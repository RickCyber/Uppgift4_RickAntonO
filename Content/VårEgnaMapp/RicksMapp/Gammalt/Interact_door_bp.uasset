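; An interactable door Blueprint that opens and closes when the player presses E nearby, with an optional key lock.
; Box overlap enables input from player controller 0, and leaving the box disables it.
; When locked, it sends an inventory check to the overlapping actor and prints "Key Required (Locked)" if that fails.
; Otherwise DoorState picks forward or reverse play of a timeline that drives the door's relative yaw.
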(event OnComponentBeginOverlap(Box)
  (params (OverlappedComponent :type Primitive%20Component%20Object%20Reference) (OtherActor :type Actor%20Object%20Reference) (OtherComp :type Primitive%20Component%20Object%20Reference) (OtherBodyIndex :type Integer) (bFromSweep :type Boolean) (SweepResult :type Hit%20Result%20Structure%20%28by%20ref%29))
  (Input|EnableInput (Game|GetPlayerController 0)))

(event OnComponentEndOverlap(Box)
  (params (OverlappedComponent :type Primitive%20Component%20Object%20Reference) (OtherActor :type Actor%20Object%20Reference) (OtherComp :type Primitive%20Component%20Object%20Reference) (OtherBodyIndex :type Integer))
  (Input|DisableInput (Game|GetPlayerController 0)))

(event Input|KeyboardEvents|E
  (params (Key :type Key%20Structure))
  (:Pressed
    (if (Variables|Default|GetDoorLocked)
      (bind _pickedup (Class|InventoryInterface|CheckInventory(Message) (stale OnComponentBeginOverlap(Box) OtherActor)))
      (if _pickedup
        (if (Variables|Default|GetDoorState) :!label _label
          (Variables|Default|SetDoorState false)
          (bind _doorrot (Timeline|DoorRotation Play)
            (:Update
              (Transformation|SetRelativeRotation (Variables|Default|GetDoor) (Math|Rotator|MakeRotator 0.0 0.0 _doorrot) false false)))
          (else
            (Variables|Default|SetDoorState true)
            (Timeline|DoorRotation Reverse)))
        (else
          (Development|PrintString "Key Required (Locked)" true true "(R=10.000000,G=0.000000,B=0.000000,A=1.000000)")))
      (else
        (goto _label)))))

(fn ConstructionScript)