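; Lift (hiss) Blueprint that moves its Cone component back and forth between its relative origin and EndLocation.
; The LiftMovement timeline drives a position lerp, with play rate set from TravelTime at BeginPlay.
; LiftForward starts the cycle but is not called at BeginPlay; each finish waits StopDelay, then reverses direction indefinitely.
; The construction script places the Cone at EndLocation when TestEndLocation is set, previewing the travel end point.
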(event Custom|LiftForward
  (bind (_direction _liftmovement) (Timeline|LiftMovement PlayFromStart)
    (:Update
      (Transformation|SetRelativeLocation (Variables|Default|GetCone) (Math|Vector|Lerp(Vector) "0, 0, 0" (Variables|Default|GetEndLocation) _liftmovement) false false))
    (:Finished
      (Utilities|FlowControl|Delay (Variables|Default|GetStopDelay))
      (switch Utilities|FlowControl|Switch|SwitchonETimelineDirection _direction
        (:Forward
          (CallFunction|LiftBackward))
        (:Backward
          (CallFunction|LiftForward))))))

(event Custom|LiftBackward
  (bind (_direction _liftmovement) (Timeline|LiftMovement ReverseFromEnd)
    (:Update
      (Transformation|SetRelativeLocation (Variables|Default|GetCone) (Math|Vector|Lerp(Vector) "0, 0, 0" (Variables|Default|GetEndLocation) _liftmovement) false false))
    (:Finished
      (Utilities|FlowControl|Delay (Variables|Default|GetStopDelay))
      (switch Utilities|FlowControl|Switch|SwitchonETimelineDirection _direction
        (:Forward
          (CallFunction|LiftBackward))
        (:Backward
          (CallFunction|LiftForward))))))

(event EventBeginPlay
  (Components|Timeline|SetPlayRate (Variables|Default|GetLiftMovement) (/ 1.0 (Variables|Default|GetTravelTime))))

(fn ConstructionScript
  (Transformation|SetRelativeLocation (Variables|Default|GetCone) (Math|Vector|SelectVector (Variables|Default|GetEndLocation) "0, 0, 0" (Variables|Default|GetTestEndLocation)) false false))