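; A speed boost pickup Blueprint that grants the overlapping ThirdPersonCharacter a timed boost.
; On overlap it hides the mesh, turns off its light, plays an explosion sound at the world origin and calls SpeedBostBegin on the character.
; After SpeedBostDuration it calls SpeedBostEnd and destroys itself.
; A Hovering timeline for bobbing the mesh exists but is never run.
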(event OnComponentBeginOverlap(StaticMesh)
  (params (OverlappedComponent :type Primitive%20Component%20Object%20Reference) (OtherActor :type Actor%20Object%20Reference) (OtherComp :type Primitive%20Component%20Object%20Reference) (OtherBodyIndex :type Integer) (bFromSweep :type Boolean) (SweepResult :type Hit%20Result%20Structure%20%28by%20ref%29))
  (bind _asthird_person_character (Utilities|Casting|CastToThirdPersonCharacter OtherActor))
  (bind _output_get (Variables|Default|SetActivator _asthird_person_character))
  (Development|SetHiddeninGame (Variables|Default|GetStaticMesh) true false)
  (Rendering|Components|Light|SetIntensity (Variables|Default|GetPointLight) 0.0)
  (Default|SpeedBostBegin _output_get)
  (Audio|PlaySoundatLocation "/Game/StarterContent/Audio/Explosion01.Explosion01" "0, 0, 0" "0, 0, 0" 1.0 1.0 0.0 0 0 0)
  (Utilities|FlowControl|Delay (Variables|Default|GetSpeedBostDuration))
  (Default|SpeedBostEnd _output_get)
  (Actor|DestroyActor))

(fn ConstructionScript)